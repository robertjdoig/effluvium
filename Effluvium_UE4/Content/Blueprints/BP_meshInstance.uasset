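; Actor Blueprint that spawns a straight row of mesh copies through an InstancedStaticMesh component.
; On BeginPlay a loop calls AddInstance repeatedly, stepping each copy along Y at a fixed spacing.
; Each instance transform is built from the component's world location, rotation and scale, with only the Y location offset.
; The construction script is empty, so the row is created only at runtime.
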(event EventBeginPlay
  (bind _self self)
  (bind _instancedstaticmesh (Variables|Default|GetInstancedStaticMesh _self))
  (bind _returnvalue (Transformation|GetWorldTransform _instancedstaticmesh))
  (for _index (range 0 10)
    (Components|InstancedStaticMesh|AddInstance (Variables|Default|GetInstancedStaticMesh) (Math|Transform|MakeTransform (Math|Vector|MakeVector (.x (.location _returnvalue)) (+ (.y (.location _returnvalue)) (Math|Conversions|ToFloat(Integer) (* _index 100))) (.z (.location _returnvalue))) (.rotation _returnvalue) (.scale _returnvalue)))))

(event Collision|EventActorBeginOverlap
  (params (OtherActor :type Actor%20Object%20Reference)))

(event EventTick
  (params (DeltaSeconds :type Float%20%28single-precision%29)))

(fn ConstructionScript)