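; BP_2D_Fluid is a procedural mesh scaffold for a water surface, with no fluid simulation in its graphs.
; The construction script builds a section of the MWater mesh from the Vertics6x6 and Triangles6x6 arrays.
; Tick resubmits the same vertex array to that section every frame, without modifying it in this Blueprint.
; A higher-resolution 24x24 vertex and triangle set is present but unused.
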(event EventBeginPlay)

(event Collision|EventActorBeginOverlap
  (params (OtherActor :type Actor%20Object%20Reference)))

(event EventTick
  (params (DeltaSeconds :type Float%20%28single-precision%29))
  (Class|ProceduralMeshComponent|UpdateMeshSectionLinearColor (Variables|Default|Getm_water) 0 (Variables|Default|GetVertics6x6 self)))

(fn ConstructionScript
  (bind _self self)
  (Class|ProceduralMeshComponent|CreateMeshSectionLinearColor (Variables|Default|Getm_water) 0 (Variables|Default|GetVertics6x6 _self) (Variables|Default|GetTriangles6x6 _self) 0 0 0 0 false))